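; Fire area-of-effect actor that damages actors caught in its area, built on a parent AOE class.
; On BeginPlay it binds to the inherited overlap event and sends each reported actor a small fixed damage message through a damage info struct.
; On Trigger it runs the parent logic, then attaches a scaled fire particle emitter to its root.
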(event `self.ReceiveBeginPlay`
  (`parent.ReceiveBeginPlay`)
  (add `self.OnAOEOverlapActor` (delegate `AOEOverlapActor`)))

(event `AOEOverlapActor` :!signature `self.OnAOEOverlapActor`
  (params (Actor :type "Actor Object Reference"))
  (message `/Game/DamageSystem/BPI_Damagable.TakeDamage` Actor (make `/Game/DamageSystem/S_DamageInfo` 5.0)))

(event `self.Trigger`
  (`parent.Trigger`)
  (`GameplayStatics.SpawnEmitterAttached` "/Game/StarterContent/Particles/P_Fire.P_Fire" (`self.DefaultSceneRoot`) "None" (0.0 0.0 0.0) (struct) (3.0 3.0 1.0)))

(fn `UserConstructionScript`
  (`parent.UserConstructionScript`))