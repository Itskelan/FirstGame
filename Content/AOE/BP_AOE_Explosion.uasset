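; Explosion area-of-effect actor that knocks back characters caught in its area.
; On BeginPlay it runs the parent logic, then binds a handler to the OnAOEOverlapActor dispatcher.
; The handler ignores non-Characters and launches Characters along a fixed world-space diagonal, overriding horizontal velocity and adding to vertical, rather than pushing radially from the blast center.
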(event `self.ReceiveBeginPlay`
  (`parent.ReceiveBeginPlay`)
  (add `/Game/AOE/BP_AOE_Base.OnAOEOverlapActor` (delegate `AOEOverlap`)))

(event `AOEOverlap`
  (params (Actor :type "Actor Object Reference"))
  (bind _ascharacter (cast `Character` Actor))
  (`Character.LaunchCharacter` _ascharacter (500.0 500.0 500.0) true false))

(fn `UserConstructionScript`
  (`parent.UserConstructionScript`))