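; Enemy AI pawn that chases the player and plays a crowbar melee attack on reaching its target.
; BeginPlay and PawnSensing sightings trigger an AI MoveTo aimed at the player controller rather than its pawn.
; On arrival, a CanAttack flag gates the montage until it completes or is interrupted.
; A debug-drawn forward sphere trace runs as the attack starts, but its hits are unused, so no damage is applied.
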(event `self.ReceiveBeginPlay`
  (`self.Chase Player`))

(event `Chase Player`
  (bind _returnvalue (`self.K2_GetActorLocation`))
  (`|AIMoveTo` self (0.0 0.0 0.0) (`GameplayStatics.GetPlayerController` 0) 100.0
    (:`OnSuccess`
      (if (`self.canAttack`)
        (`|PlayMontage` (`self.Mesh`) "/Game/Characters/WhiteClown/Animations/Attack/A_Crowbar_Attack_Montage.A_Crowbar_Attack_Montage"
          (:`then`
            (set `self.canAttack` false)
            (bind (_outhits _returnvalue_2) (`KismetSystemLibrary.SphereTraceMulti` :`Start` _returnvalue :`End` (+ _returnvalue (* (`KismetMathLibrary.GetForwardVector` (`self.K2_GetActorRotation`)) 180.0)) :`Radius` 20.0 :`TraceChannel` "TraceTypeQuery3" :`DrawDebugType` "ForDuration" :`DrawTime` 0.5))
            (if _returnvalue_2
              _))
          (:`OnCompleted`
            (set `self.canAttack` true :!label _label))
          (:`OnInterrupted`
            (goto _label)))))))

(event `self.PawnSensing.OnSeePawn`
  (params (Pawn :type "Pawn Object Reference"))
  (`self.Chase Player`))

(fn `UserConstructionScript`)